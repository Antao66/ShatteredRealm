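; Anim notify state that sends named custom event messages to the owning actor over a window of an animation.
; On begin and on end, it checks whether the mesh owner implements BPI_ExamplesInterface and calls NotifyCustomEventMessage with EventNameBegin or EventNameEnd respectively.
; Each handler returns true when the message is sent and false when the owner lacks the interface.
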(fn `Received_NotifyBegin`
  (params (MeshComp :type "SkeletalMeshComponent Object Reference") (Animation :type "AnimSequenceBase Object Reference") (TotalDuration :type "Float (double-precision)"))
  (returns (ReturnValue :type Boolean))
  (bind _returnvalue (`ActorComponent.GetOwner` MeshComp))
  (if (`KismetSystemLibrary.DoesImplementInterface` _returnvalue "/Game/AGR_EXAMPLES/Blueprints/Interfaces/BPI_ExamplesInterface.BPI_ExamplesInterface_C")
    (message `/Game/AGR_EXAMPLES/Blueprints/Interfaces/BPI_ExamplesInterface.NotifyCustomEvent` _returnvalue (`self.EventNameBegin`))
    (return true)
    (else
      (return false))))

(fn `Received_NotifyEnd`
  (params (MeshComp :type "SkeletalMeshComponent Object Reference") (Animation :type "AnimSequenceBase Object Reference"))
  (returns (ReturnValue :type Boolean))
  (bind _returnvalue (`ActorComponent.GetOwner` MeshComp))
  (if (`KismetSystemLibrary.DoesImplementInterface` _returnvalue "/Game/AGR_EXAMPLES/Blueprints/Interfaces/BPI_ExamplesInterface.BPI_ExamplesInterface_C")
    (message `/Game/AGR_EXAMPLES/Blueprints/Interfaces/BPI_ExamplesInterface.NotifyCustomEvent` _returnvalue (`self.EventNameEnd`))
    (return true)
    (else
      (return false))))