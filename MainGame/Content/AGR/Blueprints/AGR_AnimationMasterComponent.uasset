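; Character animation component that manages networked montages, pose tags, aim offset, turn rotation and ragdoll for its owning Character.
; Setup events set values locally and forward them to server RPCs; the turn tag's OnRep maps to movement rotation flags.
; Tick computes aim from a camera trace or control rotation and relays it via server, turns past an angle threshold, and moves the capsule to the ragdolled pelvis.
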(event `self.ReceiveBeginPlay`
  ;[0.07812 1 0] Start - references
  (bind _ascharacter (cast `Character` (`self.GetOwner`))
    (:`then`
      (bind _output_get (set `self.CharacterReference` _ascharacter))
      (set `self.CharMovementComponent` (`Character.CharacterMovement` _output_get))
      (`KismetSystemLibrary.Delay` 0.0)
      (bind _ascharacter_2 (cast `Character` (`self.GetOwner`)))
      (bind _output_get_2 (set `self.CharacterReference` _ascharacter_2))
      (set `self.CharMovementComponent` (`Character.CharacterMovement` _output_get_2)))
    (:`CastFailed`
      (`KismetSystemLibrary.PrintString` "Cast to character failed!"))))

(event `ServerAimOffset`
  (params (Aim :type "Rotator Structure"))
  ;[0 1 0.282] TICK
  (`self.MultiAimOffset` Aim))

(event `MultiAimOffset`
  (params (AimOffset :type "Rotator Structure"))
  (bind _characterreference (`self.CharacterReference`))
  ;[0 1 0.282] TICK
  (`/Engine/EditorBlueprintResources/StandardMacros.IsValid` _characterreference
    (:`Is Valid`
      (if (not (and (`Pawn.IsLocallyControlled` _characterreference) (`Pawn.IsPlayerControlled` _characterreference)))
        (set `self.AimOffset` AimOffset)))))

(event `self.ReceiveTick`
  (params (DeltaSeconds :type "Float (single-precision)"))
  (bind _returnvalue (`GameplayStatics.GetPlayerCameraManager` 0))
  (bind _debug_ (`self.Debug?`))
  (bind _characterreference (`self.CharacterReference`))
  (bind _characterreference_2 (`self.CharacterReference`))
  (bind _charmovementcomponent (`self.CharMovementComponent`))
  (bind _returnvalue_2 (`PlayerCameraManager.GetCameraLocation` _returnvalue))
  (bind _returnvalue_3 (`KismetMathLibrary.FClamp` (`self.TurnTolerance`) 1.0 90.0))
  (bind _mesh (`Character.Mesh` (`self.CharacterReference`)))
  (bind _returnvalue_4 (`SceneComponent.GetSocketLocation` _mesh "head"))
  (bind _returnvalue_5 (`SceneComponent.GetSocketLocation` _mesh "ik_hand_gun"))
  (bind (_returnvalue_roll _returnvalue_pitch _returnvalue_yaw) (`KismetMathLibrary.BreakRotator` (`KismetMathLibrary.NormalizedDeltaRotator` (`self.AimOffset`) (`Actor.K2_GetActorRotation` (`self.CharacterReference`)))))
  (bind _returnvalue_6 (`SceneComponent.GetSocketLocation` (`Character.Mesh` (`self.CharacterReference`)) (select `bool` (== (`self.AimOffsetTag`) (struct)) :`false` "spine_03" :`true` "ik_hand_gun" :!type "Name")))
  (bind _returnvalue_7 (+ _returnvalue_2 (* (`Actor.GetActorForwardVector` _returnvalue) 10000.0)))
  ;[0 1 0.282] TICK
  (`|ExecutionSequence`
    (:`then_0`
      (if (`Pawn.IsLocallyControlled` _characterreference)
        (if (and (`Pawn.IsPlayerControlled` _characterreference) (`self.CameraBasedAim?`))
          (bind (_outhit _returnvalue_8) (`KismetSystemLibrary.LineTraceSingle` _returnvalue_2 _returnvalue_7 "TraceTypeQuery1" true (`|MakeArray` (`self.GetOwner`)) (select `bool` (`self.Debug?`) :`true` "ForOneFrame" :!type "EDrawDebugTrace Enum")))
          (if _returnvalue_8
            (set `self.LookAtLocation` (`.Location` (`GameplayStatics.BreakHitResult` _outhit)))
            (bind _output_get (set `self.AimOffset` (`KismetMathLibrary.FindLookAtRotation` _returnvalue_6 (`.Location` (`GameplayStatics.BreakHitResult` _outhit)))))
            (`self.ServerAimOffset` _output_get)
            (if _debug_
              (`KismetSystemLibrary.DrawDebugLine` _returnvalue_4 (`.Location` (`GameplayStatics.BreakHitResult` _outhit)) (struct :`G` 0.5 :`B` 0.5 :`A` 1.0) 0.0 1.0)
              (`KismetSystemLibrary.DrawDebugLine` _returnvalue_5 (`.Location` (`GameplayStatics.BreakHitResult` _outhit)) (struct :`R` 0.5 :`B` 0.5 :`A` 1.0) 0.0 1.0))
            (else
              (bind _output_get_2 (set `self.AimOffset` (`KismetMathLibrary.FindLookAtRotation` _returnvalue_6 _returnvalue_7)))
              (`self.ServerAimOffset` _output_get_2)
              (if _debug_
                (`KismetSystemLibrary.DrawDebugLine` _returnvalue_4 _returnvalue_7 (struct :`G` 0.5 :`B` 0.5 :`A` 1.0) 0.0 1.0)
                (`KismetSystemLibrary.DrawDebugLine` _returnvalue_5 _returnvalue_7 (struct :`R` 0.5 :`B` 0.5 :`A` 1.0) 0.0 1.0))))
          (else
            (bind _output_get_3 (set `self.AimOffset` (`Pawn.GetControlRotation` _characterreference)))
            (`self.ServerAimOffset` _output_get_3)))))
    (:`then_1`
      (if (== (`self.RotateTurnTag`) (struct :`TagName` "Animation.Turn.DesiredRotAtAngle"))
        (if (or (> (`KismetMathLibrary.Abs` _returnvalue_yaw) (`self.TurnStartAngle`)) (> (`KismetMathLibrary.VSize` (`Actor.GetVelocity` (`self.CharacterReference`))) 50.0))
          (set `CharacterMovementComponent.bUseControllerDesiredRotation` true _charmovementcomponent)
          (elif (`KismetMathLibrary.InRange_FloatFloat` _returnvalue_yaw (/ _returnvalue_3 -1.0) (/ _returnvalue_3 1.0))
            (set `CharacterMovementComponent.bUseControllerDesiredRotation` false _charmovementcomponent)))))
    (:`then_2`
      (if (`self.IsRagdolling`)
        (`Actor.K2_SetActorLocation` _characterreference_2 (+ (`SceneComponent.GetSocketLocation` (`Character.Mesh` _characterreference_2) "pelvis") (`KismetMathLibrary.MakeVector` 0.0 0.0 (/ (`CapsuleComponent.GetScaledCapsuleHalfHeight` (`Character.CapsuleComponent` _characterreference_2)) 2.0))) false true)))))

(event `ServerPlayMontage`
  (params (MontageToPlay :type "AnimMontage Object Reference") (PlayRate :type "Float (double-precision)") (StartingSection :type Name))
  ;[0 1 0.7422] Multiplayer Animation Montage
  (`Character.PlayAnimMontage` (`self.CharacterReference`) MontageToPlay PlayRate StartingSection)
  (`self.MultiPlayMontage` MontageToPlay PlayRate StartingSection))

(event `PlayNetworkedMontage`
  (params (Montage :type "AnimMontage Object Reference") (PlayRate :type "Float (double-precision)" :default 1.0) (StartingSection :type Name))
  ;[0 1 0.7422] Multiplayer Animation Montage
  (if (`self.LocalPlayer`)
    (`Character.PlayAnimMontage` (`self.CharacterReference`) Montage PlayRate StartingSection)
    (`self.ServerPlayMontage` Montage PlayRate StartingSection)))

(event `MultiPlayMontage`
  (params (AnimMontage :type "AnimMontage Object Reference") (InPlayRate :type "Float (double-precision)") (StartSectionName :type Name))
  ;[0 1 0.7422] Multiplayer Animation Montage
  (if (not (`self.LocalPlayer`))
    (`Character.PlayAnimMontage` (`self.CharacterReference`) AnimMontage InPlayRate StartSectionName)))

(event `EventSetupFirstPerson`
  (params (`IsFirstPersonView?` :type Boolean))
  ;[0.1953 1 0] FP View
  (bind _output_get (set `self.IsFirstPersonView?` `IsFirstPersonView?`))
  (`self.OnFPPChange` _output_get))

(event `EventSetupBasePose`
  (params (BasePoseTag :type "GameplayTag Structure"))
  ;[1 0.375 0] Set Base pose
  (set `self.BasePoseTag` BasePoseTag)
  (`self.ServerSetBasePose` BasePoseTag))

(event `ServerSetBasePose`
  (params (BasePoseTag :type "GameplayTag Structure"))
  ;[1 0.375 0] Set Base pose
  (set `self.BasePoseTag` BasePoseTag))

(event `EventSetupOverlayPose`
  (params (OverlayTag :type "GameplayTag Structure"))
  ;[1 0 0.8203] Set OverlayPose
  (set `self.OverlayTag` OverlayTag)
  (`self.ServerSetOverlayPose` OverlayTag))

(event `ServerSetOverlayPose`
  (params (OverlayTag :type "GameplayTag Structure"))
  ;[1 0 0.8203] Set OverlayPose
  (set `self.OverlayTag` OverlayTag))

(event `ServerSetRotation`
  (params (RotateTurnTag :type "GameplayTag Structure" :default (struct)) (RotationSpeed :type "Float (double-precision)" :default 380.0) (TurnStartAngle :type "Float (double-precision)" :default 90.0) (TurnTolerance :type "Float (double-precision)" :default 5.0))
  ;[0 0.0625 1] Change Rotation
  (set `self.RotateTurnTag` RotateTurnTag)
  (set `self.RotationSpeed` RotationSpeed)
  (set `self.TurnStartAngle` TurnStartAngle)
  (set `self.TurnTolerance` TurnTolerance))

(event `EventSetupTurnRotation`
  (params (RotationType :type "GameplayTag Structure") (RotationSpeed :type "Float (double-precision)") (TurnStartAngle :type "Float (double-precision)") (TurnTolerance :type "Float (double-precision)"))
  ;[0 0.0625 1] Change Rotation
  (set `self.RotateTurnTag` RotationType)
  (set `self.RotationSpeed` RotationSpeed)
  (set `self.TurnStartAngle` TurnStartAngle)
  (set `self.TurnTolerance` TurnTolerance)
  (`self.ServerSetRotation` RotationType RotationSpeed TurnStartAngle TurnTolerance))

(event `ServerSetAimOffset`
  (params (AimOffsetTag :type "GameplayTag Structure") (AimOffsetSpeed :type "Float (double-precision)" :default 6.0) (AimOffsetClampAbsValue :type "Float (double-precision)") (`CameraBased?` :type Boolean))
  ;[0 1 0.5547] Set aim offset
  (set `self.AimOffsetTag` AimOffsetTag)
  (set `self.AimOffsetSpeed` AimOffsetSpeed)
  (set `self.AimOffsetClampAbsValue` AimOffsetClampAbsValue)
  (set `self.CameraBasedAim?` `CameraBased?`))

(event `EventSetupAimOffset`
  (params (AimOffsetTag :type "GameplayTag Structure" :default (struct)) (AimOffsetSpeed :type "Float (double-precision)" :default 6.0) (AimOffsetClampAbsValue :type "Float (double-precision)" :default 90.0) (`CameraBasedAim?` :type Boolean))
  ;[0 1 0.5547] Set aim offset
  (set `self.AimOffsetTag` AimOffsetTag)
  (set `self.AimOffsetSpeed` AimOffsetSpeed)
  (set `self.AimOffsetClampAbsValue` AimOffsetClampAbsValue)
  (set `self.CameraBasedAim?` `CameraBasedAim?`)
  (`self.ServerSetAimOffset` AimOffsetTag AimOffsetSpeed AimOffsetClampAbsValue `CameraBasedAim?`))

(event `ServerRagdoll`
  (params (Condition :type Boolean))
  (bind _characterreference (`self.CharacterReference`))
  (bind _mesh (`Character.Mesh` _characterreference))
  (bind _mesh_2 (`Character.Mesh` (`self.CharacterReference`)))
  (bind _capsulecomponent (`Character.CapsuleComponent` _characterreference))
  ;[0.7812 1 0] Ragdoll
  (bind _output_get (set `self.IsRagdolling` Condition))
  (if _output_get
    ;;[0 0.2969 1] Simulate
    (`SkeletalMeshComponent.SetAllBodiesBelowSimulatePhysics` _mesh_2 (stale `Ragdoll` InBoneName) true true :!label _label)
    (`SkeletalMeshComponent.SetAllBodiesBelowPhysicsBlendWeight` _mesh_2 (stale `Ragdoll` InBoneName) (stale `Ragdoll` PhysicsBlendWeight) false true)
    (`KismetSystemLibrary.Delay` 0.2)
    (`CharacterMovementComponent.SetMovementMode` (`self.CharMovementComponent`) "MOVE_Custom" 0)
    (else
      ;;[0.7812 0 1] End
      (`AnimInstance.SavePoseSnapshot` (`SkeletalMeshComponent.GetAnimInstance` (`Character.Mesh` (`self.CharacterReference`))) "RagdollPose" :!label _label_2)
      (`SkeletalMeshComponent.SetAllBodiesSimulatePhysics` _mesh false)
      (`SceneComponent.K2_AttachToComponent` _mesh _capsulecomponent "None" "SnapToTarget" "SnapToTarget" "KeepWorld" true)
      (`SceneComponent.K2_SetRelativeLocationAndRotation` _mesh (`KismetMathLibrary.MakeVector` 0.0 0.0 (* (`CapsuleComponent.CapsuleHalfHeight` _capsulecomponent) -1.0)) (struct :`Yaw` -90.0) false false)
      (`CharacterMovementComponent.SetMovementMode` (`self.CharMovementComponent`) "MOVE_Walking" 0))))

(event `Ragdoll`
  (params (`Start?` :type Boolean) (InBoneName :type "Name (by ref)") (PhysicsBlendWeight :type "Float (double-precision)"))
  ;[0.7812 1 0] Ragdoll
  (bind _output_get (set `self.IsRagdolling` `Start?`))
  (if _output_get
    ;;[0 0.2969 1] Simulate
    (`self.ServerRagdoll` `Start?`)
    (goto _label)
    (else
      ;;[0.7812 0 1] End
      (`self.ServerRagdoll` `Start?`)
      (goto _label_2))))

(fn `IsFirstPerson?`
  (returns (`FppView?` :type Boolean))
  (return (`self.IsFirstPersonView?`)))

(fn `LocalPlayer`
  (returns (IsLocalPlayer :type Boolean))
  (bind _characterreference (`self.CharacterReference`))
  (return (and (`Pawn.IsLocallyControlled` _characterreference) (`Pawn.IsPlayerControlled` _characterreference))))

(fn `OnRep_IsRagdolling`
  (`self.Ragdoll` (`self.IsRagdolling`) "pelvis" 1.0))

(fn `OnRep_RotateTurnTag`
  (bind _charmovementcomponent (`self.CharMovementComponent`))
  (bind _charmovementcomponent_2 (`self.CharMovementComponent`))
  (bind _charmovementcomponent_3 (`self.CharMovementComponent`))
  (bind _charmovementcomponent_4 (`self.CharMovementComponent`))
  (bind _charmovementcomponent_5 (`self.CharMovementComponent`))
  (`/Engine/EditorBlueprintResources/StandardMacros.IsValid` (`self.CharacterReference`)
    (:`Is Valid`
      (`/Engine/EditorBlueprintResources/StandardMacros.IsValid` (`self.CharMovementComponent`)
        (:`Is Valid`
          (`|SwitchGameplayTag` (`self.RotateTurnTag`)
            (:`Animation.Turn.NONE`
              (set `Pawn.bUseControllerRotationYaw` false (`self.CharacterReference`))
              (set `CharacterMovementComponent.bOrientRotationToMovement` false _charmovementcomponent_4)
              (set `CharacterMovementComponent.bUseControllerDesiredRotation` false _charmovementcomponent_4))
            (:`Animation.Turn.CharacterRotYaw`
              (set `Pawn.bUseControllerRotationYaw` true (`self.CharacterReference`))
              (set `CharacterMovementComponent.bOrientRotationToMovement` false _charmovementcomponent_2)
              (set `CharacterMovementComponent.bUseControllerDesiredRotation` false _charmovementcomponent_2))
            (:`Animation.Turn.DesiredRotation`
              (set `Pawn.bUseControllerRotationYaw` false (`self.CharacterReference`))
              (set `CharacterMovementComponent.bOrientRotationToMovement` false _charmovementcomponent_3)
              (set `CharacterMovementComponent.bUseControllerDesiredRotation` true _charmovementcomponent_3))
            (:`Animation.Turn.RotToMovement`
              (set `Pawn.bUseControllerRotationYaw` false (`self.CharacterReference`))
              (set `CharacterMovementComponent.bOrientRotationToMovement` true _charmovementcomponent)
              (set `CharacterMovementComponent.bUseControllerDesiredRotation` false _charmovementcomponent))
            (:`Animation.Turn.DesiredRotAtAngle`
              (set `Pawn.bUseControllerRotationYaw` false (`self.CharacterReference`))
              (set `CharacterMovementComponent.bOrientRotationToMovement` false _charmovementcomponent_5)
              (set `CharacterMovementComponent.bUseControllerDesiredRotation` false _charmovementcomponent_5))))))))