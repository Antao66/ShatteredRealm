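; BP_EnemyBase is a base enemy Blueprint that tracks health and reacts to damage.
; Health starts at MaxHealth on BeginPlay, and AnyDamage subtracts incoming damage from it.
; When health reaches zero or below, it calls the Death event, which currently only prints a message.
; Death has no guard, so further hits after death trigger it again.
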(event `self.ReceiveBeginPlay`
  ;[1 0 0.3047] Begin Play
  (set `self.Health` (`self.MaxHealth`)))

(event `self.ReceiveAnyDamage`
  (params (Damage :type "Float (single-precision)") (DamageType :type "DamageType Object Reference") (InstigatedBy :type "Controller Object Reference") (DamageCauser :type "Actor Object Reference"))
  ;[0 0.2266 1] Receiving Damage
  (set `self.Health` (- (`self.Health`) Damage))
  (if (<= (`self.Health`) 0.0)
    (`self.Death`)))

(event `Death`
  ;[0.8047 0 1] Death
  (`KismetSystemLibrary.PrintString` "Enemy is dead"))

(fn `UserConstructionScript`)