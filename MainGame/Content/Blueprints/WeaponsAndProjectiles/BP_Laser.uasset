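; BP_Laser is a laser projectile that damages actors tagged Enemy.
; It plays a sound at its location on BeginPlay.
; On Hit, it applies fixed damage to tagged enemies with its owner as damage causer, and destroys itself whatever it struck.
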(event `self.ReceiveBeginPlay`
  ;[1 0 0.1875] Begin Play
  (`GameplayStatics.PlaySoundAtLocation` null (`self.K2_GetActorLocation`) (struct) 1.0 1.0 0.0 null null null))

(event `self.ReceiveHit`
  (params (MyComp :type "PrimitiveComponent Object Reference") (Other :type "Actor Object Reference") (OtherComp :type "PrimitiveComponent Object Reference") (bSelfMoved :type Boolean) (HitLocation :type "Vector Structure") (HitNormal :type "Vector Structure") (NormalImpulse :type "Vector Structure") (Hit :type "HitResult Structure (by ref)"))
  ;[0 0.625 1] Hit Something
  ;;[1 0 0.5625] Hitting an Enemy
  (if (`self.ActorHasTag` Other "Enemy")
    (`GameplayStatics.ApplyDamage` Other 25.0 null (`self.GetOwner`))
    (`self.K2_DestroyActor`)
    (else
      (`self.K2_DestroyActor`))))

(fn `UserConstructionScript`)