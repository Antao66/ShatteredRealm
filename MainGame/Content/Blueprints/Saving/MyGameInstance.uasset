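; Game instance that owns the player's save data and handles saving, loading and deleting it in a single slot.
; On Init it loads the existing MySaveGame from the slot or creates a new one.
; Saving writes the BP_TDController character's location and a hardcoded "Main" name to disk; loading teleports the character using only the in-memory location.
; Clearing deletes the slot but leaves the in-memory data intact.
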(event `self.ReceiveInit`
  (bind _saveslotname (`self.SaveSlotName`))
  (bind _returnvalue (`GameplayStatics.DoesSaveGameExist` _saveslotname))
  (if _returnvalue
    (bind _returnvalue_2 (`GameplayStatics.LoadGameFromSlot` _saveslotname))
    (bind _asmy_save_game (cast `/Game/Blueprints/Saving/MySaveGame` _returnvalue_2))
    (set `self.SaveGameData` _asmy_save_game)
    (else
      (bind _returnvalue_3 (`GameplayStatics.CreateSaveGameObject` "/Game/Blueprints/Saving/MySaveGame.MySaveGame_C"))
      (set `self.SaveGameData` _returnvalue_3))))

(fn `ClearSaveData`
  (`GameplayStatics.DeleteGameInSlot` (`self.SaveSlotName`)))

(fn `LoadPlayerData`
  (locals (player :type "/Game/Blueprints/BP_TDController Object Reference"))
  (bind _savedata_location (break `/Game/Blueprints/Saving/SaveData` (`/Game/Blueprints/Saving/MySaveGame.SaveData` (`self.SaveGameData`))))
  (bind _asbp_tdcontroller (cast `/Game/Blueprints/BP_TDController` (`GameplayStatics.GetPlayerCharacter` 0)))
  (bind _output_get (set `local.player` _asbp_tdcontroller))
  (`Actor.K2_SetActorLocation` _output_get _savedata_location false false))

(fn `SavePlayerData`
  (locals (player :type "/Game/Blueprints/BP_TDController Object Reference"))
  (bind _savegamedata (`self.SaveGameData`))
  (bind _asbp_tdcontroller (cast `/Game/Blueprints/BP_TDController` (`GameplayStatics.GetPlayerCharacter` 0)))
  (bind _output_get (set `local.player` _asbp_tdcontroller))
  (set `/Game/Blueprints/Saving/MySaveGame.SaveData` (make `/Game/Blueprints/Saving/SaveData` (`Actor.K2_GetActorLocation` _output_get) "Main") _savegamedata)
  (`GameplayStatics.SaveGameToSlot` _savegamedata (`self.SaveSlotName`)))