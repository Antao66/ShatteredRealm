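; BP_HealingSalve is a health pickup that restores the player's health on contact.
; On actor overlap, it checks for the Player tag and casts the other actor to BP_TDController.
; It adds HealAmount to that actor's Health, capped at MaxHealth, then destroys itself.
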(event `self.ReceiveActorBeginOverlap`
  (params (OtherActor :type "Actor Object Reference"))
  (if (`self.ActorHasTag` OtherActor "Player")
    (bind _asbp_tdcontroller (cast `/Game/Blueprints/Player/BP_TDController` OtherActor))
    (bind _returnvalue (+ (`self.HealAmount`) (`/Game/Blueprints/Player/BP_TDController.Health` _asbp_tdcontroller)))
    (bind _maxhealth (`/Game/Blueprints/Player/BP_TDController.MaxHealth` _asbp_tdcontroller))
    (if (>= _returnvalue _maxhealth)
      (set `/Game/Blueprints/Player/BP_TDController.Health` _maxhealth _asbp_tdcontroller)
      (`self.K2_DestroyActor`)
      (else
        (set `/Game/Blueprints/Player/BP_TDController.Health` _returnvalue _asbp_tdcontroller)
        (`self.K2_DestroyActor`)))))

(fn `UserConstructionScript`)